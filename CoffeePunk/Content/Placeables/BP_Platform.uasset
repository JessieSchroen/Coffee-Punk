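; BP_Platform is a placeable 2D platform whose length is set by Size and built from Paper2D sprites.
; The construction script pins the actor's world X to 100, then adds grouped sprite instances: a left cap, evenly spaced centre tiles and an offset right cap.
; When Size is not positive, a half-width piece replaces the centre tiles.
; The event graph holds only disabled placeholder events, so the platform has no runtime logic.
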(fn `UserConstructionScript`
  (bind (_returnvalue_x _returnvalue_y _returnvalue_z) (`KismetMathLibrary.BreakVector` (`self.K2_GetActorLocation` self)))
  (bind _returnvalue (> (`self.Size`) 0))
  (`self.K2_SetActorLocation` (`KismetMathLibrary.MakeVector` 100.0 _returnvalue_y _returnvalue_z) false true)
  (switch `int` (`self.Size`)
    (:`Default`
      (`PaperGroupedSpriteComponent.AddInstance` (`self.PaperGroupedSprite`) (`KismetMathLibrary.MakeTransform` (0.0 0.0 0.0)) "/Game/Art/Platform/SPR_PlatformLeft.SPR_PlatformLeft" false (struct :`R` 1.0 :`G` 1.0 :`B` 1.0 :`A` 1.0))
      (if _returnvalue
        (for _index (range (`self.Size`))
          (`PaperGroupedSpriteComponent.AddInstance` (`self.PaperGroupedSprite`) (`KismetMathLibrary.MakeTransform` (`KismetMathLibrary.MakeVector` (* _index 300))) "/Game/Art/Platform/Sprite_PlatformCentre.Sprite_PlatformCentre" false (struct :`R` 1.0 :`G` 1.0 :`B` 1.0 :`A` 1.0)))
        (else
          (`PaperGroupedSpriteComponent.AddInstance` (`self.PaperGroupedSprite`) (`KismetMathLibrary.MakeTransform` (0.0 0.0 0.0)) "/Game/Art/Platform/Sprite_PlatformHalf.Sprite_PlatformHalf" false (struct :`R` 1.0 :`G` 1.0 :`B` 1.0 :`A` 1.0))))
      (`PaperGroupedSpriteComponent.AddInstance` (`self.PaperGroupedSprite`) (`KismetMathLibrary.MakeTransform` (`KismetMathLibrary.MakeVector` (+ (* (`self.Size`) (`KismetMathLibrary.SelectInt` 300 150 _returnvalue)) (`KismetMathLibrary.SelectInt` 0 150 _returnvalue)))) "/Game/Art/Platform/Sprite_PlatformRight.Sprite_PlatformRight" false (struct :`R` 1.0 :`G` 1.0 :`B` 1.0 :`A` 1.0)))))