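; BP_Elevator is a placeable Paper2D elevator that moves a platform sprite along a horizontal or vertical chain track.
; The construction script pins the actor to a fixed X depth, builds the track from grouped sprite instances scaled by Size, and picks the platform sprite by ElevatorType.
; On BeginPlay, a timeline paced by TravelTime drives the platform's offset, using arithmetic on the type enum instead of a branch to choose the axis.
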(event `self.ReceiveBeginPlay`
  (bind _elevatortype (`self.ElevatorType`))
  (bind _returnvalue (- _elevatortype 1))
  (`TimelineComponent.SetPlayRate` (`self.AnimMovementCurve`) (/ 1.0 (`self.TravelTime`)))
  (bind (_direction _position) (`Timeline|AnimMovementCurve`)
    (:`Update`
      (bind _returnvalue_2 (* _position (* (`self.Size`) 300.0)))
      (`SceneComponent.K2_SetRelativeLocation` (`self.PaperSprite`) (`KismetMathLibrary.MakeVector` 10.0 (* (* _returnvalue_2 (* _returnvalue _returnvalue)) -1.0) (* _returnvalue_2 (+ _elevatortype 0))) false false))))

(fn `UserConstructionScript`
  (bind (_returnvalue_x _returnvalue_y _returnvalue_z) (`KismetMathLibrary.BreakVector` (`self.K2_GetActorLocation` self)))
  (`self.K2_SetActorLocation` (`KismetMathLibrary.MakeVector` 100.0 _returnvalue_y _returnvalue_z) false true)
  (switch `EOrientation` (`self.ElevatorType`)
    (:`Orient_Horizontal`
      ;[1 1 1] Build Horizontal
      (`PaperGroupedSpriteComponent.AddInstance` (`self.PaperGroupedSprite`) (`KismetMathLibrary.MakeTransform` (0.0 0.0 0.0)) "/Game/Art/Elevator/Sprite_ChainLeft.Sprite_ChainLeft" false (struct :`R` 1.0 :`G` 1.0 :`B` 1.0 :`A` 1.0))
      (for _index (range (`self.Size`))
        (`PaperGroupedSpriteComponent.AddInstance` (`self.PaperGroupedSprite`) (`KismetMathLibrary.MakeTransform` (`KismetMathLibrary.MakeVector` (* _index 300))) "/Game/Art/Elevator/Sprite_ChainHorizontal.Sprite_ChainHorizontal" false (struct :`R` 1.0 :`G` 1.0 :`B` 1.0 :`A` 1.0)))
      (`PaperGroupedSpriteComponent.AddInstance` (`self.PaperGroupedSprite`) (`KismetMathLibrary.MakeTransform` (`KismetMathLibrary.MakeVector` (* (`self.Size`) 300))) "/Game/Art/Elevator/Sprite_ChainRight.Sprite_ChainRight" false (struct :`R` 1.0 :`G` 1.0 :`B` 1.0 :`A` 1.0))
      (`PaperSpriteComponent.SetSprite` (`self.PaperSprite`) "/Game/Art/Elevator/Sprite_ElevatorHorizontal.Sprite_ElevatorHorizontal"))
    (:`Orient_Vertical`
      ;[1 1 1] Build Verticle
      (`PaperGroupedSpriteComponent.AddInstance` (`self.PaperGroupedSprite`) (`KismetMathLibrary.MakeTransform` (0.0 0.0 0.0)) "/Game/Art/Elevator/Sprite_ChainBottom.Sprite_ChainBottom" false (struct :`R` 1.0 :`G` 1.0 :`B` 1.0 :`A` 1.0))
      (for _index_2 (range (`self.Size`))
        (`PaperGroupedSpriteComponent.AddInstance` (`self.PaperGroupedSprite`) (`KismetMathLibrary.MakeTransform` (`KismetMathLibrary.MakeVector` 0.0 0.0 (* _index_2 300))) "/Game/Art/Elevator/Sprite_ChainVerticle.Sprite_ChainVerticle" false (struct :`R` 1.0 :`G` 1.0 :`B` 1.0 :`A` 1.0)))
      (`PaperGroupedSpriteComponent.AddInstance` (`self.PaperGroupedSprite`) (`KismetMathLibrary.MakeTransform` (`KismetMathLibrary.MakeVector` 0.0 0.0 (* (`self.Size`) 300))) "/Game/Art/Elevator/Sprite_ChainTop.Sprite_ChainTop" false (struct :`R` 1.0 :`G` 1.0 :`B` 1.0 :`A` 1.0))
      (`PaperSpriteComponent.SetSprite` (`self.PaperSprite`) "/Game/Art/Elevator/Sprite_ElevatorVerticle.Sprite_ElevatorVerticle"))))