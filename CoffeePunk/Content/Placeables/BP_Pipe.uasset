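; Grid-placed 2D pipe piece that rotates in quarter turns, with straight, elbow, tee, cross and valve types plus locked variants.
; Construction snaps it to a 128-unit Y/Z grid, then applies the sprite and direction for its type.
; Locked types are flagged at BeginPlay, blocking in-game rotation and highlight tint while staying orientable in the editor.
; QueryPipeDirection offsets the type's base layout by current direction and returns it with the cell.
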(event `self.ReceiveBeginPlay`
  ;[1 1 1] Prevent Rotation of locked pipes AFTER game has started
  (if (> (`self.PipeType`) 4)
    (set `self.IsLocked` true)
    (else
      (set `self.IsLocked` false))))

(event `self.ReceiveTick`
  (params (DeltaSeconds :type "Float (single-precision)")))

(fn `Highlight`
  (params (IsHighlighted :type Boolean))
  (bind _pipesprite (`self.PipeSprite`))
  (bind _output_get (set `self.IsHighlighted` IsHighlighted))
  (if _output_get
    (if (`self.IsLocked`)
      (`PaperSpriteComponent.SetSpriteColor` _pipesprite (`self.BaseColour`) :!label _label)
      (else
        (`PaperSpriteComponent.SetSpriteColor` _pipesprite (struct :`R` 1.0 :`G` 0.874343 :`A` 1.0))))
    (else
      (goto _label))))

(fn `QueryPipeDirection`
  (returns (PipeLayout :type "/Game/Core/Structs/PipeLayoutReference Structure") (`Cell Vector` :type "/Game/Core/Structs/CellVector Structure"))
  (bind _temparray (`self.TempArray`))
  ;[1 1 1] Calculate new layout from relative rotation
  (for _array_element (`.PipeLayout_6_11AF8DD645FD4AFD3AD9748ACF5700DB` (break `/Game/Core/Structs/PipeLayoutReference` (`|GetArrayItem` (`self.BasePipeLayouts`) (`KismetMathLibrary.Conv_ByteToInt` (`self.PipeType`)))))
    (`KismetArrayLibrary.Array_Add` (`.PipeLayout_6_11AF8DD645FD4AFD3AD9748ACF5700DB` (break `/Game/Core/Structs/PipeLayoutReference` _temparray)) (cast `/Game/Core/Enums/EDirection` (mod (+ (`KismetMathLibrary.Conv_ByteToInt` _array_element) (`KismetMathLibrary.Conv_ByteToInt` (`self.PipeDirection`))) 4))))
  (return _temparray (`self.Cell`)))

(fn `Rotate`
  (params (RelativeDirection :type "/Game/Core/Enums/ERelativeDirection Enum" :default "NewEnumerator0"))
  (if (== RelativeDirection 0)
    (`GameplayStatics.PlaySound2D` "/Game/Audio/SFX/pipe_rotation_mixdown.pipe_rotation_mixdown" 0.5 1.0 0.0 null null)
    (`self.SetDirection` (cast `/Game/Core/Enums/EDirection` (mod (+ (`self.PipeDirection`) 1) 4)))
    (else
      (`GameplayStatics.PlaySound2D` "/Game/Audio/SFX/pipe_rotation_mixdown.pipe_rotation_mixdown" 0.5 1.0 0.0 null null)
      (`self.SetDirection` (cast `/Game/Core/Enums/EDirection` (mod (- (`self.PipeDirection`) 1) 4))))))

(fn `SetDirection`
  (params (Direction :type "/Game/Core/Enums/EDirection Enum" :default "NewEnumerator0"))
  (if (not (`self.IsLocked`))
    (bind _output_get (set `self.PipeDirection` Direction))
    (`SceneComponent.K2_SetRelativeRotation` (`self.Scene`) (`KismetMathLibrary.MakeRotator` (* (`KismetMathLibrary.Conv_ByteToDouble` _output_get) -90.0)) false false)))

(fn `UserConstructionScript`
  (`self.SnapToGrid` (`self.K2_GetActorLocation`)
    (:`  `
      (switch `/Game/Core/Enums/EPipeType` "NewEnumerator0"
        (:`NewEnumerator0`
          _)
        (:`NewEnumerator1`
          _)
        (:`NewEnumerator2`
          _)
        (:`NewEnumerator3`
          _)
        (:`NewEnumerator4`
          _)
        (:`NewEnumerator5`
          _)
        (:`NewEnumerator6`
          _)
        (:`NewEnumerator7`
          _)
        (:`NewEnumerator8`
          _)
        (:`NewEnumerator9`
          _))
      (`PaperSpriteComponent.SetSprite` (`self.PipeSprite`) (`|GetArrayItem` (`self.SpriteList`) (`KismetMathLibrary.Conv_ByteToInt` (`self.PipeType`))))
      (switch `/Game/Core/Enums/EDirection` "NewEnumerator0"
        (:`NewEnumerator0`
          _)
        (:`NewEnumerator1`
          _)
        (:`NewEnumerator2`
          _)
        (:`NewEnumerator3`
          _))
      (`self.SetDirection` (`self.PipeDirection`)))))